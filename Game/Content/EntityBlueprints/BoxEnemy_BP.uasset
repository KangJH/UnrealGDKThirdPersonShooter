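; BoxEnemy_BP is a networked box enemy whose cube is tinted by a replicated color, apparently tied to the worker that has authority over it.
; The construction script creates a dynamic material instance for the cube.
; When server authority changes, it sends the game mode's UnrealWorkerColor to ColorComponent.
; The component's update event sets the material's Color parameter only on the Remote branch of the authority switch.
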(event Custom|UpdateColor
  (params (Color :type Linear%20Color%20Structure))
  (Networking|SwitchHasAuthority
    (:Remote
      (Rendering|Material|SetVectorParameterValue (Variables|Default|GetColor_M) "Color" Color :!class /Script/Engine.MaterialInstanceDynamic))))

(event EventBeginPlay
  (EventDispatchers|BindEventtoOnUpdateColor (Variables|Default|GetColorComponent) (delegate Custom|UpdateColor)))

(event EventServerAuthorityChanged
  (Default|UpdateColorComponent (Variables|Default|GetColorComponent) (Variables|/Game/EntityBlueprints/TPSGameMode_BP.TPSGameMode_BP_C|GetUnrealWorker_Color (.AsTPSGame%20Mode%20BP (Utilities|Casting|CastToTPSGameMode_BP (Game|GetGameMode))))))

(fn ConstructionScript
  (bind _returnvalue (Rendering|Material|CreateDynamicMaterialInstance (Variables|Default|GetCube) 0 "/Game/Materials/BoxEnemy.BoxEnemy" "None" :!class /Script/Engine.PrimitiveComponent))
  (Variables|Default|SetColor_M _returnvalue))